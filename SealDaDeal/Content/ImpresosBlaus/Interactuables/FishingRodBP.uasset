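; Clickable fishing rod actor that adds fish to the player's count until a limit is reached.
; Hovering over its static mesh switches the mouse cursor to a hand, and leaving restores crosshairs.
; Each click increments and prints FishNum on the TopDownCharacter, or destroys the rod instead if that count has already reached five.
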(event `self.StaticMeshComponent.OnBeginCursorOver`
  (params (TouchedComponent :type "PrimitiveComponent Object Reference"))
  (set `PlayerController.CurrentMouseCursor` "Hand" (`GameplayStatics.GetPlayerController` 0)))

(event `self.StaticMeshComponent.OnEndCursorOver`
  (params (TouchedComponent :type "PrimitiveComponent Object Reference"))
  (set `PlayerController.CurrentMouseCursor` "Crosshairs" (`GameplayStatics.GetPlayerController` 0)))

(event `self.StaticMeshComponent.OnClicked`
  (params (TouchedComponent :type "PrimitiveComponent Object Reference") (ButtonPressed :type "Key Structure"))
  (bind _astop_down_character (cast `/Game/TopDownBP/Blueprints/TopDownCharacter` (`GameplayStatics.GetPlayerCharacter` 0)))
  (bind _fishnum (`/Game/TopDownBP/Blueprints/TopDownCharacter.FishNum` _astop_down_character))
  (if (>= _fishnum 5.0)
    (`self.K2_DestroyActor`)
    (else
      (set `/Game/TopDownBP/Blueprints/TopDownCharacter.FishNum` (+ _fishnum 1.0) _astop_down_character)
      (`KismetSystemLibrary.PrintString` (`KismetStringLibrary.Conv_DoubleToString` _fishnum)))))

(fn `UserConstructionScript`)